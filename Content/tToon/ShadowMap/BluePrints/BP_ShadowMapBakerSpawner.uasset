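; BP_ShadowMapBakerSpawner automatically gives the level's directional lights a BP_ShadowMapBaker for tToon shadow maps.
; Its construction script finds every DirectionalLight and skips any that already has a baker attached, as checked by CheckAttachedActor.
; For the rest, it creates a baker as a child actor component, passing HiddenActors and the light.
; Each baker is offset along the light's forward vector by LightDist, matches its rotation and attaches to it.
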(fn `CheckAttachedActor`
  (params (Actors :type "Array of Actor Object Reference") (TargetClass :type "Object Class Reference"))
  (returns (Result :type Boolean))
  (locals (TmpResult :type Boolean))
  (set `local.TmpResult` false)
  (for _array_element Actors
    (if (== (`GameplayStatics.GetObjectClass` _array_element) TargetClass)
      (set `local.TmpResult` true)))
  (return (`local.TmpResult`)))

(fn `UserConstructionScript`
  (bind _outactors (`GameplayStatics.GetAllActorsOfClass` "/Script/Engine.DirectionalLight"))
  (for _array_element _outactors
    (bind _result (`self.CheckAttachedActor` (`self.GetAttachedActors` _array_element) "/Game/tToon/ShadowMap/BluePrints/BP_ShadowMapBaker.BP_ShadowMapBaker_C"))
    (if (not _result)
      (bind _returnvalue (`AddComponent|NODE_AddChildActorComponent-0` :`RelativeTransform` (`KismetMathLibrary.MakeTransform` (0.0 0.0 0.0))))
      (`ChildActorComponent.SetChildActorClass` _returnvalue "/Game/tToon/ShadowMap/BluePrints/BP_ShadowMapBaker.BP_ShadowMapBaker_C")
      (bind _asbp_shadow_map_baker (cast `/Game/tToon/ShadowMap/BluePrints/BP_ShadowMapBaker` (`ChildActorComponent.ChildActor` _returnvalue) :!pure true))
      (set `/Game/tToon/ShadowMap/BluePrints/BP_ShadowMapBaker.HiddenActors` (`self.HiddenActors`) _asbp_shadow_map_baker)
      (set `/Game/tToon/ShadowMap/BluePrints/BP_ShadowMapBaker.Light` _array_element _asbp_shadow_map_baker)
      (`self.K2_SetActorLocationAndRotation` _asbp_shadow_map_baker (+ (`self.K2_GetActorLocation` _array_element) (* (`self.GetActorForwardVector` _array_element) (`self.LightDist`))) (`self.K2_GetActorRotation` _array_element) false false)
      (`SceneComponent.K2_AttachToComponent` _returnvalue (`Actor.RootComponent` _array_element) "None" "KeepWorld" "KeepWorld" "KeepWorld" true))))