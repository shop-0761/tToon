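; BP_ShadowMapBaker is a custom shadow-map actor that uses a SceneCaptureComponent2D as the light's view.
; Construction captures the scene; BeginPlay applies the hidden-actor list to the capture component.
; Construction and Tick write actor position and axes to MPC_ShadowMapBaker for materials to read.
; UpdateShadowMap passes the capture texture to TargetDynamicMaterials, but the code creating those materials and render targets is disconnected.
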(event `self.ReceiveBeginPlay`
  (set `SceneCaptureComponent.HiddenActors` (`self.HiddenActors`) (`self.SceneCaptureComponent2D`)))

(event `self.ReceiveTick`
  (params (DeltaSeconds :type "Float (single-precision)"))
  (`self.UpdateLightStatus`))

(event `UpdateLightStatus`
  (bind _returnvalue (`self.K2_GetActorRotation`))
  (`KismetMaterialLibrary.SetVectorParameterValue` "/Game/tToon/ShadowMap/MPC_ShadowMapBaker.MPC_ShadowMapBaker" "LightPostion" (`KismetMathLibrary.Conv_VectorToLinearColor` (`self.K2_GetActorLocation`)))
  (`KismetMaterialLibrary.SetVectorParameterValue` "/Game/tToon/ShadowMap/MPC_ShadowMapBaker.MPC_ShadowMapBaker" "XPlane" (`KismetMathLibrary.Conv_VectorToLinearColor` (`KismetMathLibrary.GetRightVector` _returnvalue)))
  (`KismetMaterialLibrary.SetVectorParameterValue` "/Game/tToon/ShadowMap/MPC_ShadowMapBaker.MPC_ShadowMapBaker" "YPlane" (`KismetMathLibrary.Conv_VectorToLinearColor` (`KismetMathLibrary.GetUpVector` _returnvalue)))
  (`KismetMaterialLibrary.SetVectorParameterValue` "/Game/tToon/ShadowMap/MPC_ShadowMapBaker.MPC_ShadowMapBaker" "ZPlane" (`KismetMathLibrary.Conv_VectorToLinearColor` (`KismetMathLibrary.GetForwardVector` _returnvalue))))

(event `UpdateShadowMap`
  (`MaterialInstanceDynamic.SetTextureParameterValue` (`self.TargetDynamicMaterials`) "ShadowMap" (`SceneCaptureComponent2D.TextureTarget` (`self.SceneCaptureComponent2D`))))

(fn `UserConstructionScript`
  (`SceneCaptureComponent2D.CaptureScene` (`self.SceneCaptureComponent2D`))
  (`self.UpdateLightStatus`))